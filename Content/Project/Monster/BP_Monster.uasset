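; Monster Blueprint that runs a Locomotion, Chase, Attack and Dead state machine, with an HP bar widget initialized to full.
; SetState writes the state to the AI Blackboard and sets walk speed.
; Sighting a living player or taking damage starts Chase and stores the target as Instigator and Blackboard key.
; Tick drops Chase beyond sight radius, extended once damaged, and leaves Attack when the player dies; attack-check events are empty stubs.
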(event OnSeePawn(PawnSensing)
  (params (Pawn :type Pawn%20Object%20Reference))
  ;[1 1 1] Player가 살아있다면 Chase -> Set Instigator
  (if (Utilities|Enum|Equal(Enum) (Variables|Default|GetStates) "NewEnumerator0")
    (bind _asbp_character (Utilities|Casting|CastToBP_Character Pawn))
    (if (not (Variables|/Game/Project/Player/BP_Character.BP_Character_C|GetIsDead _asbp_character))
      (CallFunction|SetState "NewEnumerator1")
      (bind _output_get (Variables|Actor|SetInstigator Pawn))
      (AI|Components|Blackboard|SetValueasObject (AI|GetBlackboard (AI|GetAIController self)) (Variables|Default|GetTargetPlayerKey) _output_get))))

(event Custom|SetState
  (params (NewState :type E_MonsterStates%20Enum :default "NewEnumerator0"))
  ;[1 1 1] Set Monster States
  (if (Utilities|Enum|NotEqual(Enum) (Variables|Default|GetStates) "NewEnumerator3")
    (if (Utilities|Enum|NotEqual(Enum) (Variables|Default|GetStates) NewState)
      (bind _output_get (Variables|Default|SetStates NewState))
      (AI|Components|Blackboard|SetValueasEnum (AI|GetBlackboard (AI|GetAIController self)) (Variables|Default|GetStateKey) _output_get)
      (switch Utilities|FlowControl|Switch|SwitchonE_MonsterStates (Variables|Default|GetStates)
        (:NewEnumerator0
          (Variables|/Script/Engine.CharacterMovementComponent|SetMaxWalkSpeed (Variables|Character|GetCharacterMovement) 2e+02))
        (:NewEnumerator1
          (Variables|/Script/Engine.CharacterMovementComponent|SetMaxWalkSpeed (Variables|Character|GetCharacterMovement) 4e+02))
        (:NewEnumerator2
          (Variables|/Script/Engine.CharacterMovementComponent|SetMaxWalkSpeed (Variables|Character|GetCharacterMovement) 0.0 :!label _label))
        (:NewEnumerator3
          (goto _label))))))

(event Custom|OnChase
  ;[1 1 1] Chase -> Locomotion
  (Utilities|IsValid (Variables|Actor|GetInstigator)
    (:Is%20Valid
      (if (Variables|Default|GetIsDamaged)
        (if (> (Math|Vector|Distance(Vector) (Transformation|GetActorLocation (Variables|Actor|GetInstigator)) (Transformation|GetActorLocation)) (* (Variables|/Script/AIModule.PawnSensingComponent|GetSightRadius (Variables|Default|GetPawnSensing)) 3.0))
          (Variables|Actor|SetInstigator 0)
          (CallFunction|SetState "NewEnumerator0")
          (Variables|Default|SetIsDamaged false))
        (elif (> (Math|Vector|Distance(Vector) (Transformation|GetActorLocation (Variables|Actor|GetInstigator)) (Transformation|GetActorLocation)) (Variables|/Script/AIModule.PawnSensingComponent|GetSightRadius (Variables|Default|GetPawnSensing)))
          (Variables|Actor|SetInstigator 0)
          (CallFunction|SetState "NewEnumerator0"))))))

(event Custom|OnLocomotion)

(event Custom|OnAttack
  ;[1 1 1] Attack -> Locomotion
  (Utilities|IsValid (Variables|Actor|GetInstigator)
    (:Is%20Valid
      (bind _asbp_character (Utilities|Casting|CastToBP_Character (Variables|Actor|GetInstigator)))
      (if (Variables|/Game/Project/Player/BP_Character.BP_Character_C|GetIsDead _asbp_character)
        (CallFunction|SetState "NewEnumerator0")
        (Variables|Actor|SetInstigator 0)))))

(event Custom|AttackCheckBegin)

(event Custom|AttackCheckEnd)

(event Game|Damage|EventAnyDamage
  (params (Damage :type Float%20%28single-precision%29) (DamageType :type Damage%20Type%20Object%20Reference) (InstigatedBy :type Controller%20Object%20Reference) (DamageCauser :type Actor%20Object%20Reference))
  ;[1 1 1] 플레이어가 공격하면 -> Chase
  (Variables|Default|SetIsDamaged true)
  (CallFunction|SetState "NewEnumerator1")
  (bind _asbp_character (Utilities|Casting|CastToBP_Character DamageCauser))
  (bind _output_get (Variables|Actor|SetInstigator _asbp_character))
  (AI|Components|Blackboard|SetValueasObject (AI|GetBlackboard (AI|GetAIController self)) (Variables|Default|GetTargetPlayerKey) _output_get))

(event EventTick
  (params (DeltaSeconds :type Float%20%28single-precision%29))
  ;[1 1 1] Tic마다 State에 해당하는 이벤트 호출
  (switch Utilities|FlowControl|Switch|SwitchonE_MonsterStates (Variables|Default|GetStates)
    (:NewEnumerator0
      (CallFunction|OnLocomotion))
    (:NewEnumerator1
      (CallFunction|OnChase))
    (:NewEnumerator2
      (CallFunction|OnAttack))))

(event EventBeginPlay
  ;[1 1 1] Initialize HBBar / HPPercent
  (bind _aswbp_hphud (Utilities|Casting|CastToWBP_HPHUD (UserInterface|GetUserWidgetObject (Variables|Default|GetHPBar))))
  (bind _output_get (Variables|Default|SetHPHUD _aswbp_hphud))
  (Default|SetHPPercent _output_get 1.0)
  (Rendering|SetCastShadow (Variables|Default|GetHPBar) false))

(fn ConstructionScript)