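; BP_DarkStorm is the actor for the Dark Storm skill, dealing damage to actors that begin overlapping its Attack component.
; On each overlap it looks up the DarkStorm row in DT_Skill and applies that row's Damage to the other actor, with no filtering.
; The first player controller is passed as both event instigator and damage causer.
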(event OnComponentBeginOverlap(Attack)
  (params (OverlappedComponent :type Primitive%20Component%20Object%20Reference) (OtherActor :type Actor%20Object%20Reference) (OtherComp :type Primitive%20Component%20Object%20Reference) (OtherBodyIndex :type Integer) (bFromSweep :type Boolean) (SweepResult :type Hit%20Result%20Structure%20%28by%20ref%29))
  (bind _returnvalue (Game|GetPlayerController 0))
  (bind _returnvalue_2 (Utilities|GetDataTableRow "/Game/Project/Skills/DT_Skill.DT_Skill" "DarkStorm")
    (:then
      (Game|Damage|ApplyDamage OtherActor (Utilities|Struct|BreakS_Skill _returnvalue_2) _returnvalue _returnvalue))))

(event EventBeginPlay
  (|CallParentFunction))

(event Collision|EventActorBeginOverlap
  (params (OtherActor :type Actor%20Object%20Reference))
  (|CallParentFunction OtherActor) ; This node is disabled and will not be called.\nDrag off pins to build functionality.
)

(event EventTick
  (params (DeltaSeconds :type Float%20%28single-precision%29))
  (|CallParentFunction DeltaSeconds) ; This node is disabled and will not be called.\nDrag off pins to build functionality.
)

(fn ConstructionScript
  (|CallParentFunction))