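; BP_Item is an item actor that shows a pickup prompt when a BP_Character is within range.
; Its Sphere overlap events toggle the PickUpTextWidget and an IsOverlapItem flag.
; While the flag is set, Tick assigns the item to the Item variable of the player character cached at BeginPlay.
; End overlap leaves that reference in place, and the pickup itself is not handled here.
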(event OnComponentBeginOverlap(Sphere)
  (params (OverlappedComponent :type Primitive%20Component%20Object%20Reference) (OtherActor :type Actor%20Object%20Reference) (OtherComp :type Primitive%20Component%20Object%20Reference) (OtherBodyIndex :type Integer) (bFromSweep :type Boolean) (SweepResult :type Hit%20Result%20Structure%20%28by%20ref%29))
  (Utilities|Casting|CastToBP_Character OtherActor)
  (Rendering|SetVisibility (Variables|Default|GetPickUpTextWidget) true false)
  (Variables|Default|SetIsOverlapItem true))

(event OnComponentEndOverlap(Sphere)
  (params (OverlappedComponent :type Primitive%20Component%20Object%20Reference) (OtherActor :type Actor%20Object%20Reference) (OtherComp :type Primitive%20Component%20Object%20Reference) (OtherBodyIndex :type Integer))
  (Utilities|Casting|CastToBP_Character OtherActor)
  (Rendering|SetVisibility (Variables|Default|GetPickUpTextWidget) false false)
  (Variables|Default|SetIsOverlapItem false))

(event EventBeginPlay
  (bind _asbp_character (Utilities|Casting|CastToBP_Character (Game|GetPlayerCharacter 0)))
  (Variables|Default|SetPlayerCharacter _asbp_character))

(event EventTick
  (params (DeltaSeconds :type Float%20%28single-precision%29))
  (if (Variables|Default|GetIsOverlapItem)
    (Variables|/Game/Project/Player/BP_Character.BP_Character_C|SetItem (Variables|Default|GetPlayerCharacter) self)))

(fn ConstructionScript)