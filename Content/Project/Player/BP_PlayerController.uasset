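; BP_PlayerController is a player controller that owns the HUD and handles inventory menu toggling.
; On BeginPlay it creates a WBP_HUD widget, stores it and adds it to the viewport.
; The IA_Inventory Enhanced Input action drives a FlipFlop that alternately has the HUD show or remove the inventory menu, setting IsInventoryOpen to match.
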(event Input|EnhancedActionEvents|EnhancedInputActionIA_Inventory
  (params (ActionValue :type Boolean) (ElapsedSeconds :type Float%20%28double-precision%29) (TriggeredSeconds :type Float%20%28double-precision%29) (InputAction :type Input%20Action%20Object%20Reference :default "/Game/Project/Input/Actions/IA_Inventory.IA_Inventory"))
  (:Started
    (Utilities|FlowControl|FlipFlop
      (:A
        (Default|ShowInventoryMenu (Variables|Default|GetHUD))
        (Variables|Default|SetIsInventoryOpen true))
      (:B
        (Default|RemoveInventoryMenu (Variables|Default|GetHUD))
        (Variables|Default|SetIsInventoryOpen false)))))

(event EventBeginPlay
  (bind _returnvalue (UserInterface|CreateWidget "/Game/Project/UI/WBP_HUD.WBP_HUD_C" 0 0))
  (bind _output_get (Variables|Default|SetHUD _returnvalue))
  (UserInterface|Viewport|AddtoViewport _output_get 0))

(fn ConstructionScript)