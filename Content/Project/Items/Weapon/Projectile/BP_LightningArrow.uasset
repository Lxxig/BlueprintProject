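; BP_LightningArrow is a weapon projectile that deals damage to actors its capsule overlaps.
; On BeginPlay it caches its owning BP_Character and rotates along the character's start-to-target direction, with Tick retrying while that reference is invalid.
; Tick destroys it once its distance from the character's current location reaches the projectile row's Range.
; Overlaps apply Damage read from DT_Projectile without destroying the arrow.
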(event OnComponentBeginOverlap(Capsule)
  (params (OverlappedComponent :type Primitive%20Component%20Object%20Reference) (OtherActor :type Actor%20Object%20Reference) (OtherComp :type Primitive%20Component%20Object%20Reference) (OtherBodyIndex :type Integer) (bFromSweep :type Boolean) (SweepResult :type Hit%20Result%20Structure%20%28by%20ref%29))
  (bind _returnvalue (Utilities|GetDataTableRow "/Game/Project/Items/Weapon/Projectile/DT_Projectile.DT_Projectile" (.RowName (Utilities|Struct|BreakDataTableRowHandle (Variables|Default|GetDataTable))))
    (:then
      (Game|Damage|ApplyDamage OtherActor (Utilities|Struct|BreakS_Projectile _returnvalue) (Variables|Default|GetPlayerController) (Variables|Default|GetCharacter)))))

(event EventTick
  (params (DeltaSeconds :type Float%20%28single-precision%29))
  (Utilities|IsValid (Variables|Default|GetCharacter)
    (:Is%20Valid
      (if (>= (Math|Vector|Distance(Vector) (Transformation|GetActorLocation (Variables|Default|GetCharacter)) (Transformation|GetActorLocation)) (Utilities|Struct|BreakS_Projectile (Variables|/Game/Project/Player/BP_Character.BP_Character_C|GetProjectileDataTableOutRow (Variables|Default|GetCharacter))))
        (Actor|DestroyActor)))
    (:Is%20Not%20Valid
      (bind _asbp_character (Utilities|Casting|CastToBP_Character (Components|GetOwner)))
      (Variables|Default|SetCharacter _asbp_character)
      (Transformation|SetActorRotation (Math|Conversions|RotationFromXVector (- (Variables|/Game/Project/Player/BP_Character.BP_Character_C|GetTargetLocation (Variables|Default|GetCharacter)) (Variables|/Game/Project/Player/BP_Character.BP_Character_C|GetStartLocation (Variables|Default|GetCharacter))))))))

(event EventBeginPlay
  (bind _asbp_character (Utilities|Casting|CastToBP_Character (Components|GetOwner)))
  (Variables|Default|SetCharacter _asbp_character)
  (Transformation|SetActorRotation (Math|Conversions|RotationFromXVector (- (Variables|/Game/Project/Player/BP_Character.BP_Character_C|GetTargetLocation (Variables|Default|GetCharacter)) (Variables|/Game/Project/Player/BP_Character.BP_Character_C|GetStartLocation (Variables|Default|GetCharacter))))))

(fn ConstructionScript
  (|CallParentFunction))