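; BP_Mushroom is a mushroom monster that damages what its attack collision overlaps and dies through a damage receiver component.
; BeginPlay loads HP from the "Chest" row of DT_Monster, whose Damage value also drives attacks.
; The attack window enables that collision and temporarily switches monster and player capsule responses from Block to Overlap.
; Hits play a montage and update the HP HUD; death changes state, disables capsule collision and destroys the actor after a delay.
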(event OnComponentBeginOverlap(AttackCollision)
  (params (OverlappedComponent :type Primitive%20Component%20Object%20Reference) (OtherActor :type Actor%20Object%20Reference) (OtherComp :type Primitive%20Component%20Object%20Reference) (OtherBodyIndex :type Integer) (bFromSweep :type Boolean) (SweepResult :type Hit%20Result%20Structure%20%28by%20ref%29))
  ;[1 1 1] Attack Damage
  (Game|Damage|ApplyDamage OtherActor (Utilities|Struct|BreakS_Monster (Variables|Default|GetDataTableOutRow)) (Pawn|GetController) self))

(event Custom|OnDead
  ;[1 1 1] OnDead
  (CallFunction|SetState "NewEnumerator3")
  (Collision|SetCollisionEnabled (Variables|Default|GetCapsuleComponent) "NoCollision")
  (Utilities|FlowControl|Delay 1.3)
  (Actor|DestroyActor))

(event EventBeginPlay
  (|CallParentFunction)
  (bind _returnvalue (Utilities|GetDataTableRow "/Game/Project/Monster/DT_Monster.DT_Monster" "Chest")
    (:then
      (bind _output_get (Variables|Default|SetDataTableOutRow _returnvalue))
      (Variables|/Game/Project/System/Damage/BP_DamageReceiver.BP_DamageReceiver_C|SetMaxHealthPower (Variables|Default|GetBP_DamageReceiver) (Utilities|Struct|BreakS_Monster _output_get))
      (EventDispatchers|BindEventtoOnDead (Variables|Default|GetBP_DamageReceiver) (EventDispatchers|CreateEvent :!event Custom|OnDead))
      (Collision|SetCollisionEnabled (Variables|Default|GetAttackCollision) "NoCollision"))))

(event EventTick
  (params (DeltaSeconds :type Float%20%28single-precision%29))
  (|CallParentFunction DeltaSeconds) ; 지금 이 노드는 비활성 상태입니다. \n핀을 끌어서 다른 노드를 연결하면 활성화됩니다.
)

(event Game|Damage|EventAnyDamage
  (params (Damage :type Float%20%28single-precision%29) (DamageType :type Damage%20Type%20Object%20Reference) (InstigatedBy :type Controller%20Object%20Reference) (DamageCauser :type Actor%20Object%20Reference))
  (bind _bp_damagereceiver (Variables|Default|GetBP_DamageReceiver))
  (bind _hphud (Variables|Default|GetHPHUD))
  ;[1 1 1] Hit 처리
  (|CallParentFunction Damage DamageType InstigatedBy DamageCauser)
  (Default|ReceiveDamage _bp_damagereceiver Damage)
  (Animation|Montage|PlayMontage (Variables|Character|GetMesh) "/Game/Project/Monster/Mushroom/Anim/AM_Mushroom.AM_Mushroom"
    (:then
      (Default|SetHPPercent _hphud (Default|GetHPPercent _bp_damagereceiver))
      (Default|PlayTextAnimation _hphud (Math|Float|Truncate Damage)))))

(event EventAttackCheckBegin
  ;[1 1 1] Attack Collision On/Off and Capsule Collsion Preset Setting
  (|CallParentFunction)
  (Collision|SetCollisionEnabled (Variables|Default|GetAttackCollision) "QueryOnly")
  (Collision|SetCollisionResponsetoChannel (Variables|Default|GetCapsuleComponent) "ECC_GameTraceChannel1" "ECR_Overlap")
  (bind _asbp_character (Utilities|Casting|CastToBP_Character (Game|GetPlayerCharacter 0)))
  (Collision|SetCollisionResponsetoChannel (Variables|/Script/Engine.Character|GetCapsuleComponent _asbp_character) "ECC_GameTraceChannel5" "ECR_Overlap"))

(event EventAttackCheckEnd
  ;[1 1 1] Attack Collision On/Off and Capsule Collsion Preset Setting
  (|CallParentFunction)
  (Collision|SetCollisionEnabled (Variables|Default|GetAttackCollision) "NoCollision")
  (Collision|SetCollisionResponsetoChannel (Variables|Default|GetCapsuleComponent) "ECC_GameTraceChannel1" "ECR_Block")
  (bind _asbp_character (Utilities|Casting|CastToBP_Character (Game|GetPlayerCharacter 0)))
  (Collision|SetCollisionResponsetoChannel (Variables|/Script/Engine.Character|GetCapsuleComponent _asbp_character) "ECC_GameTraceChannel5" "ECR_Block"))

(fn ConstructionScript
  (|CallParentFunction))