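; BPC_MPSystem is a component that tracks its owner's mana, starting at the maximum on BeginPlay.
; UseSkill subtracts a skill's cost, flooring at zero and calling OnNotMana when empty, but does not call OnManaPowerChanged.
; GainHealthPower, despite its name, adds mana clamped to the maximum and calls OnManaPowerChanged.
; GetMPPercent returns current mana as a fraction of the maximum.
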(event Custom|UseSkill
  (params (MPCost :type Float%20%28double-precision%29))
  ;[1 1 1] 마나 비용 공식
  (Variables|Default|SetManaPower (- (Variables|Default|GetManaPower) MPCost))
  (if (<= (Variables|Default|GetManaPower) 0.0)
    (Variables|Default|SetManaPower 0.0)
    (if (== (Variables|Default|GetManaPower) 0.0)
      (Default|CallOnNotMana))))

(event Custom|GainHealthPower
  (params (GainAmount :type Float%20%28double-precision%29))
  (Variables|Default|SetManaPower (Math|Float|Clamp(Float) (+ (Variables|Default|GetManaPower) GainAmount) 0.0 (Variables|Default|GetMaxManaPower)))
  (Default|CallOnManaPowerChanged))

(event EventBeginPlay
  (Variables|Default|SetManaPower (Variables|Default|GetMaxManaPower)))

(fn GetMPPercent
  (return (/ (Variables|Default|GetManaPower) (Variables|Default|GetMaxManaPower))))